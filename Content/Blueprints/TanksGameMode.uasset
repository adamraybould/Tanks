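; Game mode for a tanks game that sets up missions and responds to their completion or failure.
; CreateMission spawns the mission actor, then places a tank of each tagged spawn point's type at that point.
; The same loop teleports the player's pawn to the player start and marks the mission ready after a delay.
; Mission events swap the MainTheme music to round-end or failure tracks, with completion also showing a level-complete widget.
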(event `self.CreateMission`
  (params (mission :type "Actor Class Reference"))
  (`|SpawnActorFromClass` mission (`self.MissionSpawn`) "Undefined" "OverrideRootScale" null null)
  (bind _outactors (`GameplayStatics.GetAllActorsWithTag` "TankSpawnPoint"))
  (for _array_element _outactors
    (bind _asbp_tank_spawn_point (cast `/Game/Blueprints/Entities/BP_TankSpawnPoint` _array_element))
    (bind _returnvalue (`self.GetTank` (`/Game/Blueprints/Entities/BP_TankSpawnPoint.TankType` _asbp_tank_spawn_point)))
    (`|SpawnActorFromClass` _returnvalue (`KismetMathLibrary.MakeTransform` (`self.K2_GetActorLocation` _asbp_tank_spawn_point) (`self.K2_GetActorRotation` _asbp_tank_spawn_point)) "Undefined" "OverrideRootScale" null null)
    (`self.ResetPlayerSpawn`)
    (`KismetSystemLibrary.Delay` 4.0)
    (set `self.isMissionReady` true)))

(event `self.ReceiveBeginPlay`
  (add `self.OnMissionComplete` (delegate `OnMissionComplete_Event`))
  (add `self.OnMissionFailed` (delegate `OnMissionFailed_Event`)))

(event `OnMissionComplete_Event`
  (`self.PlayMusic` "/Game/Assets/Audio/Music/055-Tanks-Round-End.055-Tanks-Round-End")
  (bind _returnvalue (`|CreateWidget` "/Game/Blueprints/UI/LevelCompleteWidget.LevelCompleteWidget_C"))
  (`UserWidget.AddToViewport` _returnvalue 0))

(event `OnMissionFailed_Event`
  (`self.PlayMusic` "/Game/Assets/Audio/Music/054-Tanks-Round-Failure.054-Tanks-Round-Failure"))

(fn `PlayMusic`
  (params (Music :type "SoundBase Object Reference"))
  (bind _maintheme (`self.MainTheme`))
  (`AudioComponent.SetSound` _maintheme Music)
  (`AudioComponent.Play` _maintheme 0.0))

(fn `ResetPlayerSpawn`
  (bind _returnvalue (`GameplayStatics.GetPlayerController` 0))
  (bind _returnvalue_2 (`self.K2_FindPlayerStart` _returnvalue))
  (`self.K2_SetActorTransform` (`Controller.K2_GetPawn` _returnvalue) (`KismetMathLibrary.MakeTransform` (`self.K2_GetActorLocation` _returnvalue_2) (`self.K2_GetActorRotation` _returnvalue_2)) false true))

(fn `UserConstructionScript`)