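; Base tank Blueprint that provides shared firing and death-feedback behavior.
; Fire spawns a projectile at the spawn point's location and rotation with the tank as owner, then cuts the movement component's velocity to a third.
; On BeginPlay it binds to the health component's OnDeath event, which plays a 2D death sound and stops the movement audio.
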(event `self.Fire`
  (bind _projectilespawnpoint (`self.ProjectileSpawnPoint`))
  (bind _pawnmovement (`self.PawnMovement`))
  ;[1 1 1] Fire Logic
  (`|SpawnActorFromClass` (`self.Projectile`) (`KismetMathLibrary.MakeTransform` (`SceneComponent.K2_GetComponentLocation` _projectilespawnpoint) (`SceneComponent.K2_GetComponentRotation` _projectilespawnpoint)) "Undefined" "OverrideRootScale" self null)
  (set `MovementComponent.Velocity` (/ (`MovementComponent.Velocity` _pawnmovement) (3.0 3.0 3.0)) _pawnmovement))

(event `self.ReceiveBeginPlay`
  ;[1 1 1] On Death
  (add `EntityHealth.OnDeath` (`self.EntityHealth`) (delegate `OnDeath_Event`)))

(event `OnDeath_Event`
  (params (killedActor :type "Actor Object Reference"))
  ;[1 1 1] On Death
  (`GameplayStatics.PlaySound2D` "/Game/Assets/Audio/DeathSound.DeathSound" 1.0 1.0 0.0 null null)
  (`AudioComponent.Stop` (`self.MovementAudio`)))

(fn `UserConstructionScript`)